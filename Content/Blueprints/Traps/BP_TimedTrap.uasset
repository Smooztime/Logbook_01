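; BP_TimedTrap is a trap Blueprint that runs on timers, starting in its deactivated state on BeginPlay.
; DeactivateTrap and ActivateTrap each set TrapMesh visibility and collision, then start a timer using DeactivatedTimer or ActivatedTimer respectively; the timer event targets are not shown.
; Both functions currently hide the mesh and disable its collision, so ActivateTrap never makes the trap visible or solid.
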(event EventBeginPlay
  (CallFunction|DeactivateTrap))

(fn ConstructionScript
  (|CallParentFunction))

(fn DeactivateTrap
  (Rendering|SetVisibility (Variables|Default|GetTrapMesh) false false)
  (Collision|SetCollisionEnabled (Variables|Default|GetTrapMesh) "NoCollision")
  (Utilities|Time|SetTimerbyEvent (EventDispatchers|CreateEvent :!event ActivateTrap) (Variables|Default|GetDeactivatedTimer)))

(fn ActivateTrap
  (Rendering|SetVisibility (Variables|Default|GetTrapMesh) false false)
  (Collision|SetCollisionEnabled (Variables|Default|GetTrapMesh) "NoCollision")
  (Utilities|Time|SetTimerbyEvent (EventDispatchers|CreateEvent :!event DeactivateTrap) (Variables|Default|GetActivatedTimer)))