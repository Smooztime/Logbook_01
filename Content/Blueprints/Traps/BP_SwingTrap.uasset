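; BP_SwingTrap is a trap actor that swings back and forth between a starting and a finishing rotation.
; A timeline starts on BeginPlay, and its swing track drives a lerp between the two angles that sets the actor's rotation on each update.
; When the timeline finishes, FlipDirection checks its direction and plays it the opposite way, so the swing repeats indefinitely.
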(event EventBeginPlay
  (bind (_direction _swingtrack) (Timeline|SwingTimeline Play)
    (:Update
      (Transformation|SetActorRotation (Math|Rotator|MakeRotator 0.0 (CallFunction|InterpAngle _swingtrack) 0.0)))
    (:Finished
      (CallFunction|FlipDirection _direction))))

(fn ConstructionScript
  (|CallParentFunction))

(fn InterpAngle
  (params (Alpha :type Float%20%28double-precision%29))
  (return (Math|Float|Lerp (Variables|Default|GetStartingRotation) (Variables|Default|GetFinishingRotation) Alpha)))

(fn FlipDirection
  (params (A :type ETimelineDirection%20Enum :default "Forward"))
  (if (Utilities|Enum|Equal(Enum) A "Forward")
    (Utilities|String|Reverse (Variables|Default|GetSwingTimeline))
    (else
      (Audio|Components|Audio|Play (Variables|Default|GetSwingTimeline)))))