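; BP_BoxTrap is a trap actor whose mesh moves back and forth continuously between a starting and a destination position.
; Each tick it sets the mesh's relative location by lerping between the two points with a sine of time since creation, remapped to 0–1 and scaled by MovementSpeed and Dampening.
; Movement is not swept, and the SineWaveMovement function is an unused stub returning zero.
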(event EventTick
  (params (DeltaSeconds :type Float%20%28single-precision%29))
  (Transformation|SetRelativeLocation (Variables|Default|GetTrapMesh) (Math|Vector|Lerp(Vector) (Variables|Default|GetStartingPosition) (Variables|Default|GetDestinationPosition) (/ (+ (Math|Trig|Sin(Radians) (* (/ (Actor|GetGameTimeSinceCreation) (Variables|Default|GetDampening)) (Variables|Default|GetMovementSpeed))) 1.0) 2.0)) false false))

(fn ConstructionScript
  (|CallParentFunction))

(fn SineWaveMovement
  (return 0.0))